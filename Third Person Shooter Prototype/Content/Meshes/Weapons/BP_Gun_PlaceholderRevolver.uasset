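; Placeholder revolver weapon Blueprint that supplies shot, reload and safety-off feedback.
; Reload plays the GunReload sequence, scaling its play rate by sequence length over required duration so the animation fits the requested time.
; Shoot activates the Flash effect, plays the shot sound at the Muzzle and returns the muzzle's world location to the caller.
; SafetyOff plays its sound at a given target's location.
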(event EventReload
  (params (Required%20Duration :type Float%20%28single-precision%29))
  (Components|Timeline|SetPlayRate (Variables|/Script/ActorSequence.ActorSequenceComponent|GetSequencePlayer (Variables|Default|GetGun%20Reload)) (|(SequenceDuration/RequiredDuration) (Class|TimeManagementBlueprintLibrary|ToSeconds(QualifiedFrameTime) (Media|MediaPlayer|GetDuration (Variables|/Script/ActorSequence.ActorSequenceComponent|GetSequencePlayer (Variables|Default|GetGun%20Reload)))) Required%20Duration))
  (Sequencer|Player|Play (Variables|/Script/ActorSequence.ActorSequenceComponent|GetSequencePlayer (Variables|Default|GetGun%20Reload)) :!class /Script/MovieScene.MovieSceneSequencePlayer))

(fn ConstructionScript)

(fn SafetyOff
  (params (Target :type Actor%20Object%20Reference))
  (Audio|PlaySoundatLocation "/Game/Audio/Gun/SC_SafetyOff.SC_SafetyOff" (Transformation|GetActorLocation Target) "0, 0, 0" 1.0 1.0 0.0 0 0 0))

(fn Shoot
  (bind _muzzle (Variables|Default|GetMuzzle))
  (bind _returnvalue (Transformation|GetWorldLocation _muzzle))
  (Components|Activation|Activate (Variables|Default|GetFlash) true)
  (Audio|PlaySoundatLocation "/Game/Audio/Gun/SC_RevolverShot.SC_RevolverShot" _returnvalue "0, 0, 0" 1.0 1.0 0.0 0 0 0)
  (return _returnvalue))