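; Game mode that relays gameplay events to the first player and spawns players at checkpoint-based start points.
; Camera keep-in-view and forced look-at events go to the player character, and message events go to the HUD, all through message calls.
; New-player handling maps the game instance's current checkpoint to a named player start.
; A data-table lookup for HUD messages is left disconnected.
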(event `/Game/Blueprints/GameMode/BPI_EventManager.Trigger Keep Target In View Event`
  (params (`Event Data` :type "/Game/Blueprints/Events/S_CameraKeepInViewData Structure"))
  (message `/Game/Blueprints/Camera/BPI_PlayerCamera.Set Camera Keep Target In View` (`GameplayStatics.GetPlayerCharacter` 0) `Event Data`))

(event `/Game/Blueprints/GameMode/BPI_EventManager.Trigger Camera Forced Look At Event`
  (params (Parameters :type "/Game/Blueprints/Events/S_CameraForcedLookAtData Structure"))
  (message `/Game/Blueprints/Camera/BPI_PlayerCamera.Set Forced Look At` (`GameplayStatics.GetPlayerCharacter` 0) Parameters))

(event `/Game/Blueprints/GameMode/BPI_EventManager.Trigger HUD Message Event`
  (params (`Event Name` :type Name) (`Message Parameters` :type "/Game/Blueprints/UI/Messages/S_MessageDisplay Structure"))
  (message `/Game/Blueprints/UI/Messages/BPI_MessageDisplay.Display Message(s)` (`PlayerController.GetHUD` (`GameplayStatics.GetPlayerController` 0)) `Message Parameters`))

(event `self.HandleStartingNewPlayer`
  (params (NewPlayer :type "PlayerController Object Reference"))
  (bind _checkpoint (message `/Game/Blueprints/GameMode/BPI_CheckpointSystem.Get Current Checkpoint` (`GameplayStatics.GetGameInstance`)))
  (`self.RestartPlayerAtPlayerStart` NewPlayer (`self.K2_FindPlayerStart` NewPlayer (select `/Game/Blueprints/Events/Enum_Checkpoints` _checkpoint :`NewEnumerator0` "Begin" :`NewEnumerator2` "R1_Jetpack_Pod" :`NewEnumerator3` "R1_Center" :`NewEnumerator4` "R2_Overlook" :`NewEnumerator5` "R2_Center" :`NewEnumerator6` "R2_Center"))))

(fn `UserConstructionScript`)