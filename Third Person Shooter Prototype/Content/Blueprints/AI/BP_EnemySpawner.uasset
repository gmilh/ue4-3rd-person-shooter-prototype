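; BP_EnemySpawner spawns an enemy turret at its own transform and signals the spawn with an alarm and flickering light.
; TriggerSpawning creates a BP_EnemyTurret, passes it the spawner's patrol points and turret type, fires the feedback event, then returns the new turret.
; SpawningFeedback plays the alarm sound at the spawner's location and uses a timeline to scale the RectLight intensity up to a configurable multiplier.
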(event `Spawning Feedback`
  (`GameplayStatics.PlaySoundAtLocation` "/Game/Audio/Turret/SC_Alarm.SC_Alarm" (`self.K2_GetActorLocation`) (struct) 1.0 1.0 0.0 null null null)
  (bind (_direction _alpha) (`Timeline|Light Flickering` :!via `PlayFromStart`)
    (:`Update`
      (`LightComponent.SetIntensity` (`self.RectLight`) (`KismetMathLibrary.Lerp` 0.0 (`self.Intensity Multiplier`) _alpha)))))

(fn `Trigger Spawning`
  (returns (`Spawned Actor` :type "Actor Object Reference"))
  (bind _returnvalue (`|SpawnActorFromClass` "/Game/Blueprints/AI/BP_EnemyTurret.BP_EnemyTurret_C" (`self.GetTransform`) "Undefined" "OverrideRootScale" null (`self.Patrol Points`) (`self.Type`) null))
  (`self.Spawning Feedback`)
  (return _returnvalue))

(fn `UserConstructionScript`)