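; Turret projectile actor that damages whatever it overlaps, ignoring other projectiles of its own class.
; On overlap it destroys itself, spawns a blood-wound particle and laser impact sound, then applies damage credited to its instigator's controller, with its owner as damage causer.
; An additional bullet-hit sound plays when the struck actor's instigator controller is a player controller.
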(event `self.ReceiveActorBeginOverlap`
  (params (OtherActor :type "Actor Object Reference"))
  (bind _returnvalue (`self.GetInstigatorController` OtherActor))
  (if (!= (`GameplayStatics.GetObjectClass` OtherActor) (`GameplayStatics.GetObjectClass` self))
    (`self.K2_DestroyActor`)
    (`self.Impact Feedback`)
    (`GameplayStatics.ApplyDamage` OtherActor (`self.Damage Points`) (`self.GetInstigatorController`) (`self.GetOwner`) "/Script/Engine.DamageType")
    (`/Engine/EditorBlueprintResources/StandardMacros.IsValid` _returnvalue
      (:`Is Valid`
        (if (`Controller.IsPlayerController` _returnvalue)
          (`GameplayStatics.PlaySoundAtLocation` "/Game/Audio/Gun/SC_BulletHit.SC_BulletHit" (`self.K2_GetActorLocation`) (struct) 1.0 1.0 0.0 null null null))))))

(fn `Impact Feedback`
  (`GameplayStatics.SpawnEmitterAtLocation` "/Game/VFX/PS_BloodWound.PS_BloodWound" (`self.K2_GetActorLocation`))
  (`GameplayStatics.PlaySoundAtLocation` "/Game/Audio/Turret/Laser_Attack/SC_TurretLaserImpact.SC_TurretLaserImpact" (`self.K2_GetActorLocation`) (struct) 1.0 1.0 0.0 null null null))

(fn `UserConstructionScript`)