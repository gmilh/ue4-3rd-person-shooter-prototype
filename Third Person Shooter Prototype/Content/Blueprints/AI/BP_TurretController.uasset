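; AI controller for enemy turrets that runs the turret behavior tree and feeds its blackboard.
; On begin play it copies intruder response type and sight radius from the controlled pawn through interface messages.
; On possess it binds to the pawn's damage event, and Spot Attacker records a player instigator's pawn as the spotted intruder in the blackboard.
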(event `self.ReceiveBeginPlay`
  ;[1 1 1 1 58] BEGIN PLAY
  (`self.RunBehaviorTree` "/Game/Blueprints/AI/BT_EnemyTurret.BT_EnemyTurret")
  (`self.Init Blackboard Values From Pawn`))

(event `Spot Attacker` :!signature `self.OnTakeAnyDamage`
  (params (DamagedActor :type "Actor Object Reference") (Damage :type "Float (double-precision)") (DamageType :type "DamageType Object Reference") (InstigatedBy :type "Controller Object Reference") (DamageCauser :type "Actor Object Reference"))
  ;[1 1 1] Spot Attacker
  (if (`self.IsPlayerController` InstigatedBy)
    (`BlackboardComponent.SetValueAsObject` (`self.Blackboard`) "Spotted Intruder" (`self.K2_GetPawn` InstigatedBy))))

(event `self.ReceivePossess`
  (params (PossessedPawn :type "Pawn Object Reference"))
  ;[1 1 1 1 56] ON POSSESS
  (add `self.OnTakeAnyDamage` PossessedPawn (`|CreateDelegate` :!event `Spot Attacker`)))

(fn `Init Blackboard Values From Pawn`
  (bind __ (message `/Game/Blueprints/AI/BPI_TurretPawn.Get Intruder Response Type` (`self.K2_GetPawn`)))
  (`BlackboardComponent.SetValueAsEnum` (`self.Blackboard`) "Intruder Response Type" __)
  (bind _radius (message `/Game/Blueprints/AI/BPI_TurretPawn.Get Sight Radius` (`self.K2_GetPawn`)))
  (`BlackboardComponent.SetValueAsFloat` (`self.Blackboard`) "Sight Radius" _radius))

(fn `UserConstructionScript`)