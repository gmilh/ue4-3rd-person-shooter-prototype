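; Enemy turret pawn, a flying Chaser or navmesh-bound Lookout, that reports spotted intruders to its Blackboard and exposes patrol points.
; FireatTarget rescales a telegraph timeline driving cannon glow and charge audio while aim tracks the target, then spawns a projectile.
; Damage swaps in a flashing material and blocks further hits until it ends.
; Low health adds smoke; death drops the turret, plays a sequence, explodes and spawns health orbs.
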(event OnSeePawn(PawnSensing)
  (params (Pawn :type Pawn%20Object%20Reference))
  ;[1 1 1 1 56] Handle Pawn Spotted
  (AI|Components|Blackboard|SetValueasObject (AI|GetBlackboard (Pawn|GetController)) (Utilities|Name|MakeLiteralName "Spotted Intruder") Pawn) ; Notify Blackboard
  (CallFunction|UpdateLightColour true))

(event Custom|Enable%20Damaging
  (bind _sphere (Variables|Default|GetSphere))
  ;[1 1 1 1 58] PROCESS DAMAGE RECEIVED
  (Utilities|FlowControl|DoOnce false) ; enters at Reset
)

(event Custom|Damage%20Flash%20Effect
  (for _array_element (Utilities|Array|MakeArray (Variables|Default|GetCylinder) (Variables|Default|GetSphere))
    (Utilities|Map|Add (Variables|Default|GetMesh%28s%29%20Materials) (Utilities|GetDisplayName _array_element) (Rendering|Material|GetMaterial _array_element 0)))
  (bind _returnvalue (Rendering|Material|CreateDynamicMaterialInstance "/Game/Materials/MI_FlashingDamage.MI_FlashingDamage" "None" :!class /Script/Engine.KismetMaterialLibrary))
  (Variables|Default|SetDamage%20Flashing%20Material _returnvalue)
  (for _array_element_2 (Utilities|Array|MakeArray (Variables|Default|GetCylinder) (Variables|Default|GetSphere))
    (Rendering|Material|SetMaterial _array_element_2 0 (Variables|Default|GetDamage%20Flashing%20Material)))
  (Components|Timeline|SetPlayRate (Variables|Default|GetDamaged) 3.0)
  (bind _emissive (Timeline|Damaged PlayFromStart)
    (:Update
      (Rendering|Material|SetScalarParameterValue (Variables|Default|GetDamage%20Flashing%20Material) "Emissive" (* 15 _emissive) :!class /Script/Engine.MaterialInstanceDynamic))
    (:Finished
      (for _array_element_3 (Utilities|Array|MakeArray (Variables|Default|GetCylinder) (Variables|Default|GetSphere))
        (Rendering|Material|SetMaterial _array_element_3 0 (.Value (Utilities|Map|Find (Variables|Default|GetMesh%28s%29%20Materials) (Utilities|GetDisplayName _array_element_3)))))
      (CallFunction|EnableDamaging))))

(event Custom|Destroy%20Turret
  ;[1 1 1 1 58] PROCESS DAMAGE RECEIVED
  ;;[1 1 1 1 56] Turret destruction
  (Actor|DestroyActor)
  (Effects|SpawnEmitteratLocation "/Game/StarterContent/Particles/P_Explosion.P_Explosion" (Transformation|GetActorLocation))
  (CallFunction|SpawnHealthOrbs 2))

(event EventFireatTarget
  (params (Intended%20Target :type Actor%20Object%20Reference) (Duration%20Telegraphing :type Float%20%28single-precision%29))
  (bind _beamer_socket (Variables|Default|GetBeamer%20Socket))
  ;[1 1 1 1 56] Fire at Target
  (Variables|Default|SetCurrent%20Target Intended%20Target) ; Save target reference\nto track with cannon
  (CallFunction|AdjustTimelineDuration (Variables|Default|GetTelegraphing%20Upcoming%20Shot) Duration%20Telegraphing)
  (Audio|Components|Audio|Play (Variables|Default|GetLaser%20Charge) 0.0) ; Attack Charging SFX
  ;;[1 1 1] Telegraph upcoming fire
  (bind (_direction _emissive _audio_volume) (Timeline|Telegraphing%20Upcoming%20Shot PlayFromStart)
    (:Update
      (Rendering|Material|SetScalarParameterValue (Variables|Default|GetShooting%20Telegraphing%20Material) "Emissive" (* _emissive 45.0) :!class /Script/Engine.MaterialInstanceDynamic)
      (Audio|Parameter|SetFloatParameter (Variables|Default|GetLaser%20Charge) "Volume" _audio_volume :!class /Script/Engine.AudioComponent))
    (:Finished
      (Audio|Components|Audio|Stop (Variables|Default|GetLaser%20Charge))
      (CallFunction|InstantiateProjectile)
      ;;[1 1 1] Stop tracking target
      (Variables|Default|SetCurrent%20Target 0) ; Clear Target Reference
      (Components|MoveComponentTo _beamer_socket (Variables|/Script/Engine.SceneComponent|GetRelativeLocation _beamer_socket) "0, 0, 0" true true 0.2 false) ; Return cannon to idle pose
    )))

(event Game|Damage|EventAnyDamage
  (params (Damage :type Float%20%28single-precision%29) (DamageType :type Damage%20Type%20Object%20Reference) (InstigatedBy :type Controller%20Object%20Reference) (DamageCauser :type Actor%20Object%20Reference))
  (bind _sphere (Variables|Default|GetSphere))
  ;[1 1 1 1 58] PROCESS DAMAGE RECEIVED
  (Utilities|FlowControl|DoOnce false
    (:Completed
      ;;[1 1 1] Reduce Hit Points
      (Variables|Default|SetCurrent%20Hit%20Points (- (Variables|Default|GetCurrent%20Hit%20Points) Damage))
      (AI|Navigation|StopMovement (Pawn|GetController))
      (CallFunction|ReceivedDamageFeedback)
      ;;[1 1 1 1 56] IF Hit Points depleted, stops AI and initiate pawn destruction
      (if (<= (Variables|Default|GetCurrent%20Hit%20Points) 0.0)
        (Actor|DestroyActor (Pawn|GetController))
        (CallFunction|AbortAnyAttack)
        (Pawn|Components|CharacterMovement|SetMovementMode (Variables|Character|GetCharacterMovement) "MOVE_Falling" 0)
        (CallFunction|TurretDestructionAnimation (EventDispatchers|CreateEvent :!event Custom|Destroy%20Turret))
        (CallFunction|SpawnHealthOrbs 1)
        (else
          ;;[1 1 1] ELSE IF Hit Points below tresshold, start emitting smoke
          (if (<= (Variables|Default|GetCurrent%20Hit%20Points) (/ (Variables|Default|GetDefault%20Hit%20Points) 2.0))
            (Utilities|FlowControl|DoOnce false
              (:Completed
                (Effects|SpawnEmitterAttached "/Game/StarterContent/Particles/P_Smoke.P_Smoke" _sphere "None" (Transformation|GetWorldLocation _sphere) "0, 0, 0" "1.000000,1.000000,1.000000" "KeepWorldPosition")
                (CallFunction|SpawnHealthOrbs 1)))))))))

(event EventTick
  (params (DeltaSeconds :type Float%20%28single-precision%29))
  ;[1 1 1 1 58] EVENT TICK
  (CallFunction|UpdateMeshRotation)
  (CallFunction|AimatTargetUpdate))

(event EventBeginPlay
  ;[1 1 1 1 58] BEGIN PLAY
  (CallFunction|InitHitPoints)
  (CallFunction|InitMovementMode))

(event EventUpdateLightColour
  (params (Chasing%20Intruder :type Boolean))
  ;[1 1 1 1 56] Update Light Colour
  (Rendering|Components|Light|SetLightColor (Variables|Default|GetRectLight) (Math|Color|SelectColor "(R=0.545098,G=0.000000,B=0.031373,A=1.000000)" "(R=1.000000,G=0.784323,B=0.306216,A=1.000000)" Chasing%20Intruder) true))

(event EventAbortAnyAttack
  (bind _beamer_socket (Variables|Default|GetBeamer%20Socket))
  ;[1 1 1 1 56] Fire at Target
  ;;[1 1 1] Abort charging attack
  (Rendering|Material|SetScalarParameterValue (Variables|Default|GetShooting%20Telegraphing%20Material) "Emissive" 0.0 :!class /Script/Engine.MaterialInstanceDynamic)
  (Audio|Components|Audio|Stop (Variables|Default|GetLaser%20Charge))
  ;;[1 1 1] Telegraph upcoming fire
  (bind (_direction _emissive _audio_volume) (Timeline|Telegraphing%20Upcoming%20Shot Stop)
    (:Update
      (Rendering|Material|SetScalarParameterValue (Variables|Default|GetShooting%20Telegraphing%20Material) "Emissive" (* _emissive 45.0) :!class /Script/Engine.MaterialInstanceDynamic)
      (Audio|Parameter|SetFloatParameter (Variables|Default|GetLaser%20Charge) "Volume" _audio_volume :!class /Script/Engine.AudioComponent))
    (:Finished
      (Audio|Components|Audio|Stop (Variables|Default|GetLaser%20Charge))
      (CallFunction|InstantiateProjectile)
      ;;[1 1 1] Stop tracking target
      (Variables|Default|SetCurrent%20Target 0) ; Clear Target Reference
      (Components|MoveComponentTo _beamer_socket (Variables|/Script/Engine.SceneComponent|GetRelativeLocation _beamer_socket) "0, 0, 0" true true 0.2 false) ; Return cannon to idle pose
    )))

(fn ConstructionScript
  (bind _returnvalue (Rendering|Material|CreateDynamicMaterialInstance (Variables|Default|GetCylinder) 0 "/Game/Materials/MI_Enemy_CannonCharging.MI_Enemy_CannonCharging" "None" :!class /Script/Engine.PrimitiveComponent))
  (Variables|Default|SetShooting%20Telegraphing%20Material _returnvalue)
  ;[1 1 1] Init Light Colour
  (Default|UpdateLightColour self false)
  (CallFunction|InitMeshRotation))

(fn UpdateMeshRotation
  (bind _mesh (Variables|Character|GetMesh))
  (Transformation|SetWorldRotation _mesh (Math|Interpolation|RInterpTo (Transformation|GetWorldRotation _mesh) (Transformation|GetActorRotation) (Utilities|Time|GetWorldDeltaSeconds) (Variables|Default|GetTurn%20Rate)) false false))

(fn InitMeshRotation
  (Transformation|SetWorldRotation (Variables|Character|GetMesh) (Transformation|GetActorRotation) false false))

(fn AimatTargetUpdate
  (bind _current_target (Variables|Default|GetCurrent%20Target))
  (bind _beamer_socket (Variables|Default|GetBeamer%20Socket))
  (Utilities|IsValid _current_target
    (:Is%20Valid
      (Transformation|SetWorldRotation _beamer_socket (Math|Interpolation|RInterpTo (Transformation|GetWorldRotation _beamer_socket) (Math|Rotator|FindLookatRotation (Transformation|GetWorldLocation (Variables|Default|GetBeamer%20Socket)) (+ (Transformation|GetActorLocation _current_target) (Transformation|GetVelocity))) (Utilities|Time|GetWorldDeltaSeconds) (Variables|Default|GetAim%20Rate)) false false))))

(fn InstantiateProjectile
  (bind _muzzle (Variables|Default|GetMuzzle))
  (Game|SpawnActorfromClass "/Game/Blueprints/AI/BP_TurretProjectile.BP_TurretProjectile_C" (Math|Transform|MakeTransform (Transformation|GetWorldLocation _muzzle) (Transformation|GetWorldRotation _muzzle)) "Undefined" 0 (Variables|Default|GetAttack%20Damage%20Points) 0)
  (Audio|PlaySoundatLocation "/Game/Audio/Turret/Laser_Attack/SC_TurretLaserShot.SC_TurretLaserShot" (Transformation|GetWorldLocation (Variables|Default|GetMuzzle)) "0, 0, 0" 1.0 1.0 0.0 0 0 0))

(fn InitHitPoints
  (Variables|Default|SetCurrent%20Hit%20Points (Variables|Default|GetDefault%20Hit%20Points)))

(fn InitMovementMode
  ;[1 1 1] Chaser will be in flying mode, to follow the player around the room
  ; Lookout will be confined to the navmesh of the overlook area they are positioned in
  (switch Utilities|FlowControl|Switch|SwitchonEnum_MovementType (Variables|Default|GetTurret%20Type)
    (:NewEnumerator0
      (Pawn|Components|CharacterMovement|SetMovementMode (Variables|Character|GetCharacterMovement) "MOVE_Flying" 0))))

(fn AdjustTimelineDuration
  (params (Timeline :type Timeline%20Component%20Object%20Reference) (RequiredDuration :type Float%20%28single-precision%29))
  ;[1 1 1] Adjust play rate to match required duration
  (Components|Timeline|SetPlayRate Timeline (|(TimelineDuration/(RequiredDuration*DefaultPlayRate)) (Components|Timeline|GetTimelineLength Timeline) RequiredDuration 1.0)))

(fn ReceivedDamageFeedback
  (CallFunction|DamageFlashEffect)
  (Effects|SpawnEmitteratLocation "/Game/VFX/PS_DustHit.PS_DustHit" (Transformation|GetActorLocation))
  (Audio|PlaySoundatLocation "/Game/Audio/Turret/Destroyed/SC_TurretDamaged.SC_TurretDamaged" (Transformation|GetActorLocation) "0, 0, 0" 1.0 1.0 0.0 0 0 0))

(fn TurretDestructionAnimation
  (params (Follow%20Up%20Event :type Delegate%20%28by%20ref%29))
  (bind _turret_destroyed (Variables|Default|GetTurret%20Destroyed))
  (bind _sequenceplayer (Variables|/Script/ActorSequence.ActorSequenceComponent|GetSequencePlayer _turret_destroyed))
  (Sequencer|Player|Play _sequenceplayer :!class /Script/MovieScene.MovieSceneSequencePlayer)
  (EventDispatchers|BindEventtoOnFinished _sequenceplayer Follow%20Up%20Event)
  (Audio|PlaySoundatLocation "/Game/Audio/Turret/Destroyed/SC_TurretDestroyed.SC_TurretDestroyed" (Transformation|GetActorLocation) "0, 0, 0" 1.0 1.0 0.0 0 0 0))

(fn SpawnHealthOrbs
  (params (Quantity :type Integer))
  (for _index (range 1 Quantity)
    (Game|SpawnActorfromClass "/Game/Blueprints/PlayerCharacter/BP_HealthPickups.BP_HealthPickups_C" (Math|Transform|MakeTransform (Transformation|GetActorLocation) "0, 0, 0" "0.200000,0.200000,0.200000") "AdjustIfPossibleButAlwaysSpawn" 0 0)))

(fn GetIntruderResponseType
  (return (Variables|Default|GetTurret%20Type)))

(fn GetNextPatrolPoint
  (params (Current%20Patrol%20Point :type BP%20Patrol%20Point%20Object%20Reference))
  (bind _patrol_points (Variables|Default|GetPatrol%20Points))
  (bind _returnvalue (Utilities|Array|FindItem _patrol_points Current%20Patrol%20Point))
  (bind _returnvalue_2 (+ _returnvalue 1))
  (Utilities|IsValid Current%20Patrol%20Point
    (:Is%20Valid
      (return (Utilities|Array|Get(acopy) (Variables|Default|GetPatrol%20Points) (Math|Integer|SelectInt _returnvalue_2 0 (<= _returnvalue_2 (Utilities|Array|Length (Variables|Default|GetPatrol%20Points)))))))
    (:Is%20Not%20Valid
      (return (Utilities|Array|Get(acopy) (Variables|Default|GetPatrol%20Points))))))

(fn GetSightRadius
  (return (Variables|/Script/AIModule.PawnSensingComponent|GetSightRadius (Variables|Default|GetPawnSensing))))

(fn PerformSurroundingScan
  (return 0.0))