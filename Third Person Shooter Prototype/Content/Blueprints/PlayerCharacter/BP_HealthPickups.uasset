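; Health pickup that homes in on a nearby player who needs health, heals them on contact and destroys itself.
; After a spawn delay it checks players inside its outer radius and opens a gate for new entrants.
; Players not needing health are watched through damage events until they leave.
; Tick moves it toward the target at constant speed with physics off; touching a non-healable actor clears the target and restores physics.
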(event `self.ReceiveTick`
  (params (DeltaSeconds :type "Float (single-precision)"))
  ;[1 1 1 1 58] TICK
  (`/Engine/EditorBlueprintResources/StandardMacros.IsValid` (`self.Player Target`)
    (:`Is Valid`
      ;;[1 1 1] Move health pack to target player actor
      (`self.K2_SetActorLocation` (`KismetMathLibrary.VInterpTo_Constant` (`self.K2_GetActorLocation`) (`self.K2_GetActorLocation` (`self.Player Target`)) (`GameplayStatics.GetWorldDeltaSeconds`) 2200.0) true))))

(event `self.ReceiveBeginPlay`
  ;[1 1 1 1 58] BEGIN PLAY
  ;;[1 1 1] Delay having health pack move towards player
  ;; (to let players have a good view of the object when spawned before it rushes towards them)
  (`KismetSystemLibrary.Delay` (`self.Initial Delay To Activate`))
  (`/Engine/EditorBlueprintResources/StandardMacros.IsValid` (`self.Player Target`)
    (:`Is Valid`
      _)
    (:`Is Not Valid`
      (`self.Check Nearby Actors For Target`)))
  (`self.Enable Targetting Player`))

(event `Check if Actor in Range Needs Health` :!signature `self.OnTakeAnyDamage`
  (params (DamagedActor :type "Actor Object Reference") (Damage :type "Float (double-precision)") (DamageType :type "DamageType Object Reference") (InstigatedBy :type "Controller Object Reference") (DamageCauser :type "Actor Object Reference"))
  ;[1 1 1 1 56] Actor in range takes damage
  (`self.Try Set Actor As Target` DamagedActor))

(event `self.Player Check.OnComponentBeginOverlap`
  (params (OverlappedComponent :type "PrimitiveComponent Object Reference") (OtherActor :type "Actor Object Reference") (OtherComp :type "PrimitiveComponent Object Reference") (OtherBodyIndex :type Integer) (bFromSweep :type Boolean) (SweepResult :type "HitResult Structure (by ref)"))
  ;[1 1 1 1 56] Actor enters outer raidus
  (`/Engine/EditorBlueprintResources/StandardMacros.Gate` true :!label _label
    (:`Exit`
      (`self.Try Set Actor As Target` OtherActor))))

(event `Enable Targetting Player`
  ;[1 1 1 1 56] Actor enters outer raidus
  (goto _label :!via `Open`))

(event `self.Player Check.OnComponentEndOverlap`
  (params (OverlappedComponent :type "PrimitiveComponent Object Reference") (OtherActor :type "Actor Object Reference") (OtherComp :type "PrimitiveComponent Object Reference") (OtherBodyIndex :type Integer))
  ;[1 1 1 1 56] Actor leaving the outer radius
  ;;[1 1 1] Verify the End Overlap event is accurate
  ;; (I had experience of this event being fired when a given actor was still inside)
  (if (not (`KismetArrayLibrary.Array_Contains` (`PrimitiveComponent.GetOverlappingActors` (`self.Player Check`) "/Game/Blueprints/PlayerCharacter/BP_PlayerCharacter.BP_PlayerCharacter_C") OtherActor))
    ;;[1 1 1] Terminate listening for damage events on the actor leaving
    (remove `self.OnTakeAnyDamage` OtherActor (`|CreateDelegate` :!event `Check if Actor in Range Needs Health`))))

(event `self.StaticMesh.OnComponentBeginOverlap`
  (params (OverlappedComponent :type "PrimitiveComponent Object Reference") (OtherActor :type "Actor Object Reference") (OtherComp :type "PrimitiveComponent Object Reference") (OtherBodyIndex :type Integer) (bFromSweep :type Boolean) (SweepResult :type "HitResult Structure (by ref)"))
  ;[1 1 1 1 56] Actor overlaps pickup
  (if (`KismetSystemLibrary.DoesImplementInterface` OtherActor "/Game/Blueprints/PlayerCharacter/Interfaces/BPI_Healable.BPI_Healable_C")
    (bind ____ (message `/Game/Blueprints/PlayerCharacter/Interfaces/BPI_Healable.Does Need Health` OtherActor))
    (if ____
      (message `/Game/Blueprints/PlayerCharacter/Interfaces/BPI_Healable.Gain Health` OtherActor (`self.Health Points Gained`))
      (`self.K2_DestroyActor`))
    (else
      (set `self.Player Target` null)
      (`PrimitiveComponent.SetSimulatePhysics` (`self.StaticMesh`) true))))

(fn `Check Nearby Actors For Target`
  (for _array_element (`PrimitiveComponent.GetOverlappingActors` (`self.Player Check`) "/Game/Blueprints/PlayerCharacter/BP_PlayerCharacter.BP_PlayerCharacter_C")
    (`self.Try Set Actor As Target` _array_element)))

(fn `Try Set Actor As Target`
  (params (`Actor to Check` :type "Actor Object Reference"))
  (locals (`Actor being checked` :type "Actor Object Reference"))
  (bind _output_get (set `local.Actor being checked` `Actor to Check`))
  (bind ____ (message `/Game/Blueprints/PlayerCharacter/Interfaces/BPI_Healable.Does Need Health` _output_get))
  (if ____
    (set `self.Player Target` (`local.Actor being checked`))
    (`PrimitiveComponent.SetSimulatePhysics` (`self.StaticMesh`) false)
    (else
      (add `self.OnTakeAnyDamage` (`local.Actor being checked`) (`|CreateDelegate` :!event `Check if Actor in Range Needs Health`)))))

(fn `UserConstructionScript`)