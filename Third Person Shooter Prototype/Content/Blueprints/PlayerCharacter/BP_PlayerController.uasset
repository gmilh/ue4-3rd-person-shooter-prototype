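; Player controller that handles camera shakes, gamepad rumble, restarting on death and quitting.
; Any key press records whether a gamepad is in use and tells the game instance, and rumble plays only on gamepad.
; Destruction of the possessed pawn reloads the current level.
; Holding Quit through a retriggerable delay exits the game, with a gate closed on release to cancel it.
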(event `/Game/Blueprints/PlayerCharacter/Interfaces/BPI_PlayerFeedback.Play Camera Shake`
  (params (Shake :type "CameraShake Class Reference"))
  ;[1 1 1] Play Camera Shakes
  (`PlayerCameraManager.PlayCameraShake` :`self` (`self.PlayerCameraManager`) :`ShakeClass` Shake))

(event `Key|AnyKey` :consume false :overrideparent false
  (params (Key :type "Key Structure"))
  ;[1 1 1] Detect Input Device
  (:`Pressed`
    (set `self.Using Gamepad` (`KismetInputLibrary.Key_IsGamepadKey` Key))
    (message `/Game/Blueprints/UI/BPI_InputDeviceType.Set Using Gamepad` (`GameplayStatics.GetGameInstance`) (`self.Using Gamepad`))))

(event `/Game/Blueprints/PlayerCharacter/Interfaces/BPI_PlayerFeedback.Play Rumble Effect`
  (params (`Force Feedback` :type "ForceFeedbackEffect Object Reference"))
  ;[1 1 1] Play Rumble Effects (only when using Gamepad)
  (if (`self.Using Gamepad`)
    (`self.K2_ClientPlayForceFeedback` `Force Feedback` "None" false true)))

(event `self.ReceivePossess`
  (params (PossessedPawn :type "Pawn Object Reference"))
  (add `self.OnDestroyed` PossessedPawn (delegate `Game Over`)))

(event `Game Over` :!signature `self.OnDestroyed`
  (params (DestroyedActor :type "Actor Object Reference"))
  (bind _returnvalue (`GameplayStatics.GetCurrentLevelName` true))
  (`GameplayStatics.OpenLevel` (`KismetStringLibrary.Conv_StringToName` _returnvalue)))

(event `InputAction|Quit`
  (params (Key :type "Key Structure"))
  (:`Pressed`
    (`|ExecutionSequence`
      (:`then_0`
        (`KismetSystemLibrary.RetriggerableDelay` 1.38)
        (`/Engine/EditorBlueprintResources/StandardMacros.Gate` true :!label _label
          (:`Exit`
            (`KismetSystemLibrary.QuitGame` self "Quit"))))
      (:`then_1`
        (goto _label :!via `Open`))))
  (:`Released`
    (goto _label :!via `Close`)))

(fn `UserConstructionScript`)